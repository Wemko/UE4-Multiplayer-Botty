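; Bullet pickup spawn effect actor that plays sound and sparks when it appears near the player.
; On BeginPlay it checks the distance to the first player pawn, converted to meters through the world scale.
; Within five meters it plays the audio component and activates the spark particles, then deactivates them after a short delay.
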(event `self.ReceiveBeginPlay`
  (bind _p_sparks (`self.P_Sparks`))
  (if (<= (/ (`self.GetDistanceTo` self (`GameplayStatics.GetPlayerPawn` 0)) (`HeadMountedDisplayFunctionLibrary.GetWorldToMetersScale`)) 5.0)
    (`AudioComponent.Play` (`self.Audio`) 0.0)
    (`ActorComponent.Activate` _p_sparks false)
    (`KismetSystemLibrary.Delay` 2.0)
    (`ActorComponent.Deactivate` _p_sparks)))

(fn `UserConstructionScript`)