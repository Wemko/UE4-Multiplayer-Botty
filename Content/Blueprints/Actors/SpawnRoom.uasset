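; Spawn room actor that gives its player weapon selection and a rotating door.
; On authority, the first character to enter SpawnBox while none is assigned becomes SpawnedPlayer; that player's later entries show weapon select and exits remove it.
; DoorInsideBox overlaps tell that player whether door interaction is available.
; RotateDoorRemote plays or reverses a timeline based on current door yaw, scaling its output to a 90-degree swing.
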(event `self.SpawnBox.OnComponentEndOverlap`
  (params (OverlappedComponent :type "PrimitiveComponent Object Reference") (OtherActor :type "Actor Object Reference") (OtherComp :type "PrimitiveComponent Object Reference") (OtherBodyIndex :type Integer))
  (bind _spawnedplayer (`self.SpawnedPlayer`))
  (`/Engine/EditorBlueprintResources/ActorMacros.Switch Has Authority`
    (:`Authority`
      (if (== OtherActor _spawnedplayer)
        (`/Game/ThirdPersonBP/Blueprints/ThirdPersonCharacter.RemoveWeaponSelect` _spawnedplayer)))))

(event `self.SpawnBox.OnComponentBeginOverlap`
  (params (OverlappedComponent :type "PrimitiveComponent Object Reference") (OtherActor :type "Actor Object Reference") (OtherComp :type "PrimitiveComponent Object Reference") (OtherBodyIndex :type Integer) (bFromSweep :type Boolean) (SweepResult :type "HitResult Structure (by ref)"))
  (bind _spawnedplayer (`self.SpawnedPlayer`))
  (`/Engine/EditorBlueprintResources/ActorMacros.Switch Has Authority`
    (:`Authority`
      (`self.SpawnedPlayer`
        (:`then`
          (if (== _spawnedplayer OtherActor)
            (`/Game/ThirdPersonBP/Blueprints/ThirdPersonCharacter.ShowWeaponSelect` _spawnedplayer)))
        (:`else`
          (bind _asthird_person_character (cast `/Game/ThirdPersonBP/Blueprints/ThirdPersonCharacter` OtherActor))
          (set `self.SpawnedPlayer` _asthird_person_character))))))

(event `self.DoorInsideBox.OnComponentBeginOverlap`
  (params (OverlappedComponent :type "PrimitiveComponent Object Reference") (OtherActor :type "Actor Object Reference") (OtherComp :type "PrimitiveComponent Object Reference") (OtherBodyIndex :type Integer) (bFromSweep :type Boolean) (SweepResult :type "HitResult Structure (by ref)"))
  (bind _spawnedplayer (`self.SpawnedPlayer`))
  (`/Engine/EditorBlueprintResources/ActorMacros.Switch Has Authority`
    (:`Authority`
      (if (== OtherActor _spawnedplayer)
        (`/Game/ThirdPersonBP/Blueprints/ThirdPersonCharacter.Interact with door` _spawnedplayer self true)))))

(event `self.DoorInsideBox.OnComponentEndOverlap`
  (params (OverlappedComponent :type "PrimitiveComponent Object Reference") (OtherActor :type "Actor Object Reference") (OtherComp :type "PrimitiveComponent Object Reference") (OtherBodyIndex :type Integer))
  (bind _spawnedplayer (`self.SpawnedPlayer`))
  (`/Engine/EditorBlueprintResources/ActorMacros.Switch Has Authority`
    (:`Authority`
      (if (== OtherActor _spawnedplayer)
        (`/Game/ThirdPersonBP/Blueprints/ThirdPersonCharacter.Interact with door` _spawnedplayer self false)))))

(event `Rotate Door Remote`
  (bind (_relativerotation_roll _relativerotation_pitch _relativerotation_yaw) (`KismetMathLibrary.BreakRotator` (`SceneComponent.RelativeRotation` (`self.SM_Door`))))
  (if (> _relativerotation_yaw 1.0)
    (bind (_direction _opening) (`Timeline|Timeline_0` :!label _label)
      (:`Update`
        (`SceneComponent.K2_SetRelativeRotation` (`self.SM_Door`) (`KismetMathLibrary.MakeRotator` 0.0 0.0 (* _opening 90.0)) false false)))
    (else
      (goto _label :!via `Reverse`))))

(fn `UserConstructionScript`)