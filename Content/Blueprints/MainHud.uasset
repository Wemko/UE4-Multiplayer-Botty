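; MainHud owns the player's on-screen widgets: the main interface with its score list, the chat box and the weapon selection screen.
; GetLazyInterface creates the main interface on first request, while BeginPlay waits a second for client init before adding chat and refreshing scores.
; Events show or remove weapon selection, syncing that state to MainPlayerState.
; Chat events forward messages, activation, initialization and global channel switching to the chat box.
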(event `RemoveWeaponSelect`
  (bind _currentweaponselect (`self.CurrentWeaponSelect`)
    (:`then`
      (`Widget.RemoveFromParent` _currentweaponselect)
      (set `self.CurrentWeaponSelect` null)
      (bind _asmain_player_state (cast `/Game/Blueprints/State/MainPlayerState` (`Controller.PlayerState` (`GameplayStatics.GetPlayerController` 0))))
      (`/Game/Blueprints/State/MainPlayerState.SetWeaponSelection` _asmain_player_state false))
    (:`else`)))

(event `ShowWeaponSelect`
  (`self.CurrentWeaponSelect`
    (:`then`)
    (:`else`
      (`self.GetLazyInterface`)
      (bind _returnvalue (`|CreateWidget` "/Game/Blueprints/Widgets/WeaponSelect.WeaponSelect_C"))
      (`UserWidget.AddToViewport` _returnvalue 0)
      (set `self.CurrentWeaponSelect` _returnvalue)
      (bind _asmain_player_state (cast `/Game/Blueprints/State/MainPlayerState` (`Controller.PlayerState` (`GameplayStatics.GetPlayerController` 0))))
      (`/Game/Blueprints/State/MainPlayerState.SetWeaponSelection` _asmain_player_state true))))

(event `Update Score List`
  (bind _maininterface (`self.GetLazyInterface`))
  (`/Game/Blueprints/Widgets/MainInterface.UpdateScoreList` _maininterface))

(event `self.ReceiveBeginPlay`
  (`KismetSystemLibrary.Delay` 1.0) ; Delay needed for init of client
  (`self.GetLazyInterface`)
  (bind _returnvalue (`|CreateWidget` "/Game/Blueprints/Widgets/ChatBox.ChatBox_C"))
  (bind _output_get (set `self.ChatWidget` _returnvalue))
  (`UserWidget.AddToViewport` _output_get 0)
  (`self.Update Score List`))

(event `SetChatActive`
  (`/Game/Blueprints/Widgets/ChatBox.SetChatActive` (`self.ChatWidget`)))

(event `InitializeChat`
  (bind _chatwidget (`self.ChatWidget`)
    (:`then`
      (`/Game/Blueprints/Widgets/ChatBox.InitializeChat` _chatwidget))
    (:`else`)))

(event `ReceiveMessage`
  (params (Message :type "/Game/Blueprints/Structs/ChatMessage Structure"))
  (bind _chatwidget (`self.ChatWidget`)
    (:`then`
      (`/Game/Blueprints/Widgets/ChatBox.AddChatMessage` _chatwidget Message))
    (:`else`)))

(event `SwitchGlobalChatRoom`
  (bind _chatwidget (`self.ChatWidget`)
    (:`then`
      (`/Game/Blueprints/Widgets/ChatBox.SwitchGlobalChannel` _chatwidget))
    (:`else`)))

(fn `GetLazyInterface`
  (returns (MainInterface :type "/Game/Blueprints/Widgets/MainInterface Object Reference"))
  (bind _maininterface (`self.MainInterface`)
    (:`then`
      (return _maininterface))
    (:`else`
      (bind _returnvalue (`|CreateWidget` "/Game/Blueprints/Widgets/MainInterface.MainInterface_C"))
      (`UserWidget.AddToViewport` _returnvalue 0)
      (set `self.MainInterface` _returnvalue)
      (return _returnvalue))))

(fn `UserConstructionScript`)