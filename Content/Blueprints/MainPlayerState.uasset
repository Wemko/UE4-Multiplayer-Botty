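; MainPlayerState is a player state that holds a player's score, selected weapon, ammo count and weapon-switch flag.
; Events increment the score, set the switch flag and refill ammo from the selected weapon's ammo value.
; SwitchWeaponId picks one of three hard-coded weapon structs by ID and resets the ammo count.
; WeaponSwitchEnabled has a RepNotify function, which is empty.
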(event `SetWeaponSelection`
  (params (WeaponSelection :type Boolean))
  (set `self.WeaponSwitchEnabled` WeaponSelection))

(event `IncreaseScore`
  (set `self.PlayerScore` (+ (`self.PlayerScore`) 1)))

(event `PickupAmmo`
  (bind (_selectedweapon_id _selectedweapon_delay _selectedweapon_ammo) (break `/Game/Blueprints/WeaponType` (`self.SelectedWeapon`)))
  (set `self.BulletAmount` _selectedweapon_ammo))

(event `SwitchWeaponId`
  (params (WeaponId :type Integer))
  (if (<= WeaponId 2)
    (switch `int` WeaponId
      (:`0`
        (bind _output_get (set `self.SelectedWeapon` (make `/Game/Blueprints/WeaponType` 0 0.1 10)))
        (set `self.BulletAmount` (`.ammo_8_313F725A4E3F59CE61DDD586D22F11CB` (break `/Game/Blueprints/WeaponType` _output_get))))
      (:`1`
        (bind _output_get_2 (set `self.SelectedWeapon` (make `/Game/Blueprints/WeaponType` 1 0.5 8)))
        (set `self.BulletAmount` (`.ammo_8_313F725A4E3F59CE61DDD586D22F11CB` (break `/Game/Blueprints/WeaponType` _output_get_2))))
      (:`2`
        (bind _output_get_3 (set `self.SelectedWeapon` (make `/Game/Blueprints/WeaponType` 2 1.0 5)))
        (set `self.BulletAmount` (`.ammo_8_313F725A4E3F59CE61DDD586D22F11CB` (break `/Game/Blueprints/WeaponType` _output_get_3)))))))

(fn `OnRep_WeaponSwitchEnabled`)

(fn `UserConstructionScript`)