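; MainGameState is a game state that runs a match countdown and relays global chat.
; On authority, BeginPlay sets the timer and builds the chat room map, whose two entries share one key, and Tick counts the timer down.
; SendGlobalMessage appends to the named room's message history, then forwards the message to every MainPlayerState in PlayerArray, regardless of room.
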(event `SendGlobalMessage`
  (params (Sender :type String) (Message :type Text) (ChatRoomName :type "String (by ref)"))
  (`KismetArrayLibrary.Array_Add` (`.LastMessages_10_B0267EDBD34FF635C38811B7AFA391C8` (break `/Game/Blueprints/Structs/GlobalChatRoom` (`BlueprintMapLibrary.Map_Find` (`self.ChatRooms`) ChatRoomName))) (make `/Game/Blueprints/Structs/Message` Sender Message))
  (for _array_element (`self.PlayerArray`)
    (bind _asmain_player_state (cast `/Game/Blueprints/State/MainPlayerState` _array_element))
    (`/Game/Blueprints/State/MainPlayerState.ReceiveMessage` _asmain_player_state Sender Message)))

(event `self.ReceiveBeginPlay`
  (`/Engine/EditorBlueprintResources/ActorMacros.Switch Has Authority`
    (:`Authority`
      (set `self.Time` 600.0)
      (set `self.ChatRooms` (`|MakeMap` "GlobalChatRoom1" (make `/Game/Blueprints/Structs/GlobalChatRoom` "GlobalChatRoom1") "GlobalChatRoom1" (make `/Game/Blueprints/Structs/GlobalChatRoom` "GlobalChatRoom1"))))))

(event `self.ReceiveTick`
  (params (DeltaSeconds :type "Float (single-precision)"))
  (`/Engine/EditorBlueprintResources/ActorMacros.Switch Has Authority`
    (:`Authority`
      (set `self.Time` (- (`self.Time`) DeltaSeconds)))))

(fn `UserConstructionScript`)