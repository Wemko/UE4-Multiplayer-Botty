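; Player state that holds a player's chat room view, score and weapon loadout.
; On BeginPlay it selects the game state's first chat room and initializes the HUD chat; room switches load that room's last messages, and incoming messages append only for the selected room.
; Events bump score, toggle weapon switching (with an empty OnRep), pick one of three hard-coded weapons, and refill bullets from the selected weapon's ammo.
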(event `self.ReceiveBeginPlay`
  (`self.InitilaizeChat`))

(event `InitilaizeChat`
  (bind _asmain_game_state (cast `/Game/Blueprints/State/MainGameState` (`GameplayStatics.GetGameState`)))
  (bind _output_name (break `/Game/Blueprints/Structs/GlobalChatRoom` (`|GetArrayItem` (`/Game/Blueprints/State/MainGameState.ChatRoomsArr` _asmain_game_state))))
  (set `self.SelectedGlobalChatRoom` _output_name)
  (bind _asmain_hud (cast `/Game/Blueprints/MainHud` (`PlayerController.GetHUD` (`GameplayStatics.GetPlayerController` 0))))
  (`/Game/Blueprints/MainHud.InitializeChat` _asmain_hud))

(event `ChangeChatRoom`
  (params (ChatRoomName :type String))
  (bind _asmain_game_state (cast `/Game/Blueprints/State/MainGameState` (`GameplayStatics.GetGameState`)))
  (bind (_chatroom _chatroomindex _success) (`/Game/Blueprints/State/MainGameState.GetChatRoomByName` _asmain_game_state ChatRoomName))
  (if _success
    (set `self.ChatMessages` (`.LastMessages_10_B0267EDBD34FF635C38811B7AFA391C8` (break `/Game/Blueprints/Structs/GlobalChatRoom` _chatroom)))
    (else
      (set `self.ChatMessages` (`|MakeArray` (struct) :!type "/Game/Blueprints/Structs/Message Structure"))))
  (set `self.SelectedGlobalChatRoom` ChatRoomName))

(event `ReceiveChatMessage`
  (params (Sender :type String) (Message :type Text) (ChatRoomName :type String))
  (if (`KismetStringLibrary.EqualEqual_StrStr` ChatRoomName (`self.SelectedGlobalChatRoom`))
    (`KismetArrayLibrary.Array_Add` (`self.ChatMessages`) (make `/Game/Blueprints/Structs/Message` Sender Message))))

(event `SetWeaponSelection`
  (params (WeaponSelection :type Boolean))
  (set `self.WeaponSwitchEnabled` WeaponSelection))

(event `IncreaseScore`
  (set `self.PlayerScore` (+ (`self.PlayerScore`) 1)))

(event `PickupAmmo`
  (bind (_selectedweapon_id _selectedweapon_delay _selectedweapon_ammo) (break `/Game/Blueprints/Structs/WeaponType` (`self.SelectedWeapon`)))
  (set `self.BulletAmount` _selectedweapon_ammo))

(event `SwitchWeaponId`
  (params (WeaponId :type Integer))
  (if (<= WeaponId 2)
    (switch `int` WeaponId
      (:`0`
        (bind _output_get (set `self.SelectedWeapon` (make `/Game/Blueprints/Structs/WeaponType` 0 0.1 10)))
        (set `self.BulletAmount` (`.ammo_8_313F725A4E3F59CE61DDD586D22F11CB` (break `/Game/Blueprints/Structs/WeaponType` _output_get))))
      (:`1`
        (bind _output_get_2 (set `self.SelectedWeapon` (make `/Game/Blueprints/Structs/WeaponType` 1 0.5 8)))
        (set `self.BulletAmount` (`.ammo_8_313F725A4E3F59CE61DDD586D22F11CB` (break `/Game/Blueprints/Structs/WeaponType` _output_get_2))))
      (:`2`
        (bind _output_get_3 (set `self.SelectedWeapon` (make `/Game/Blueprints/Structs/WeaponType` 2 1.0 5)))
        (set `self.BulletAmount` (`.ammo_8_313F725A4E3F59CE61DDD586D22F11CB` (break `/Game/Blueprints/Structs/WeaponType` _output_get_3)))))))

(fn `OnRep_WeaponSwitchEnabled`)

(fn `UserConstructionScript`)